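; BP_FallingPlatform is a platform that drops when the player touches it and later resets.
; BeginPlay stores the cube's starting world location and rotation.
; When BP_Player overlaps the box and CanFall is set, the cube starts simulating physics.
; After a fixed delay, it teleports back to the stored transform and physics is switched off.
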(event OnComponentBeginOverlap(Box)
  (params (OverlappedComponent :type Primitive%20Component%20Object%20Reference) (OtherActor :type Actor%20Object%20Reference) (OtherComp :type Primitive%20Component%20Object%20Reference) (OtherBodyIndex :type Integer) (bFromSweep :type Boolean) (SweepResult :type Hit%20Result%20Structure%20%28by%20ref%29))
  (Utilities|Casting|CastToBP_Player OtherActor)
  (if (Variables|Default|GetCanFall?)
    (Physics|SetSimulatePhysics (Variables|Default|GetCube) true)
    (Utilities|FlowControl|Delay 6.0)
    (Transformation|SetWorldLocationAndRotation (Variables|Default|GetCube) (Variables|Default|GetDefaultLocation) (Variables|Default|GetDefautRot) false true)
    (Physics|SetSimulatePhysics (Variables|Default|GetCube) false)))

(event Collision|EventActorBeginOverlap
  (params (OtherActor :type Actor%20Object%20Reference)))

(event EventTick
  (params (DeltaSeconds :type Float%20%28single-precision%29)))

(event EventBeginPlay
  (bind _cube (Variables|Default|GetCube))
  (Variables|Default|SetDefaultLocation (Transformation|GetWorldLocation _cube))
  (Variables|Default|SetDefautRot (Transformation|GetWorldRotation _cube)))

(fn ConstructionScript)