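; BP_Chest is a chest actor that spawns a random item when GetItem is called.
; Overlapping its Box shows the player's HUD bottom canvas with the chest's Name and registers the chest on BP_Player; leaving reverses this.
; GetItem stores a random AllChestItem entry as SelectedItem, spawns its class at ItemSpawnLoc, then destroys that spawned actor after a short delay.
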(event OnComponentBeginOverlap(Box)
  (params (OverlappedComponent :type Primitive%20Component%20Object%20Reference) (OtherActor :type Actor%20Object%20Reference) (OtherComp :type Primitive%20Component%20Object%20Reference) (OtherBodyIndex :type Integer) (bFromSweep :type Boolean) (SweepResult :type Hit%20Result%20Structure%20%28by%20ref%29))
  (bind _asbp_player (Utilities|Casting|CastToBP_Player OtherActor))
  (Default|DisplayBottomCanva (Variables|/Game/Blueprints/BP_Player.BP_Player_C|GetHUDRef _asbp_player))
  (Variables|/Game/Blueprints/WBP_HUD.WBP_HUD_C|SetName (Variables|/Game/Blueprints/BP_Player.BP_Player_C|GetHUDRef _asbp_player) (Variables|Default|GetName))
  (Variables|/Game/Blueprints/BP_Player.BP_Player_C|SetisNearChest? _asbp_player true)
  (Variables|/Game/Blueprints/BP_Player.BP_Player_C|SetChest _asbp_player self))

(event OnComponentEndOverlap(Box)
  (params (OverlappedComponent :type Primitive%20Component%20Object%20Reference) (OtherActor :type Actor%20Object%20Reference) (OtherComp :type Primitive%20Component%20Object%20Reference) (OtherBodyIndex :type Integer))
  (bind _asbp_player (Utilities|Casting|CastToBP_Player OtherActor))
  (Default|HideBottomCanva (Variables|/Game/Blueprints/BP_Player.BP_Player_C|GetHUDRef _asbp_player))
  (Variables|/Game/Blueprints/BP_Player.BP_Player_C|SetisNearChest? _asbp_player false)
  (Variables|/Game/Blueprints/BP_Player.BP_Player_C|SetChest _asbp_player 0))

(event Custom|GetItem
  (bind _output_get (Variables|Default|SetSelectedItem (.OutItem (Utilities|Array|Random (Variables|Default|GetAllChestItem)))))
  (bind _returnvalue (Game|SpawnActorfromClass (Utilities|GetClass _output_get) (Math|Transform|MakeTransform (Transformation|GetWorldLocation (Variables|Default|GetItemSpawnLoc)) "0, 0, 0" "1.000000,1.000000,1.000000") "Undefined" "MultiplyWithRoot" 0 0))
  (Utilities|FlowControl|Delay 3.0)
  (Actor|DestroyActor _returnvalue))

(event EventBeginPlay)

(fn ConstructionScript)