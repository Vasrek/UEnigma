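; Player character Blueprint with axis-driven movement and camera, checkpoint respawning, chest looting, and a HUD created at BeginPlay.
; Jump is a forward dash that launches the character while briefly hiding the mesh with Niagara effects, and Sprint lowers walk speed while held.
; Death teleports to the saved location, Win restarts the level, and debug-style keys show a flash widget or spawn projectiles.
; Timer-driven FOV zoom functions exist but are never triggered.
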(event Custom|Death
  (Transformation|SetActorLocation (Variables|Default|GetRespawnLocation) false true))

(event Custom|Checkpoint
  (params (NewRespawnLocation :type Vector))
  (Variables|Default|SetRespawnLocation NewRespawnLocation))

(event Custom|Win
  (Development|ExecuteConsoleCommand "RestartLevel" 0))

(event EventBeginPlay
  (Variables|Default|SetRespawnLocation (Transformation|GetActorLocation))
  (bind _returnvalue (UserInterface|CreateWidget "/Game/Blueprints/WBP_HUD.WBP_HUD_C"))
  (bind _output_get (Variables|Default|SetHUDRef _returnvalue))
  (UserInterface|Viewport|AddtoViewport _output_get 0)
  (Default|HideBottomCanva (Variables|Default|GetHUDRef)))

(event Input|ActionEvents|InputActionJump
  (params (Key :type Key%20Structure :default "None"))
  (bind _returnvalue (Transformation|GetActorRotation))
  (:Pressed
    (Rendering|SetVisibility (Variables|Character|GetMesh) false false)
    (AddComponent|AddNiagaraComponent false)
    (Character|LaunchCharacter (+ (* (Math|Vector|GetForwardVector _returnvalue) (Math|Conversions|ToVector(Float) 1.5e+03)) (* (Math|Vector|GetUpVector _returnvalue) (Math|Conversions|ToVector(Float) 2e+02))) false false)
    (Utilities|FlowControl|Delay 0.5)
    (Rendering|SetVisibility (Variables|Character|GetMesh) true true)
    (AddComponent|AddNiagaraComponent false)))

(event Input|ActionEvents|InputActionSprint
  (params (Key :type Key%20Structure :default "None"))
  (bind _charactermovement (Variables|Character|GetCharacterMovement))
  (:Pressed
    (Variables|/Script/Engine.CharacterMovementComponent|SetMaxWalkSpeed _charactermovement 3e+02))
  (:Released
    (Variables|/Script/Engine.CharacterMovementComponent|SetMaxWalkSpeed _charactermovement 6e+02)))

(event Input|ActionEvents|InputActionInteract
  (params (Key :type Key%20Structure :default "None"))
  (bind _chest (Variables|Default|GetChest))
  (:Pressed
    (if (Variables|Default|GetisNearChest?)
      (Default|GetItem _chest)
      (Development|PrintString (Utilities|String|ToString(Text) (Variables|/Game/Blueprints/BP_ChestItem.BP_ChestItem_C|GetName (Variables|/Game/Blueprints/BP_Chest.BP_Chest_C|GetSelectedItem _chest)))))))

(event Input|AxisEvents|InputAxisMoveForward/Backward
  (params (AxisValue :type Float%20%28single-precision%29))
  ;[1 1 1] Movement ZQSD
  (Pawn|Input|AddMovementInput (Math|Vector|GetForwardVector (Math|Rotator|MakeRotator 0.0 0.0 (.yaw (Pawn|GetControlRotation :!class /Script/Engine.Pawn)))) AxisValue false))

(event Input|AxisEvents|InputAxisMoveRight/Left
  (params (AxisValue :type Float%20%28single-precision%29))
  ;[1 1 1] Movement ZQSD
  (Pawn|Input|AddMovementInput (Math|Vector|GetRightVector (Math|Rotator|MakeRotator 0.0 0.0 (.yaw (Pawn|GetControlRotation :!class /Script/Engine.Pawn)))) AxisValue false))

(event Input|AxisEvents|InputAxisLook
  (params (AxisValue :type Float%20%28single-precision%29))
  ;[1 1 1] Camera
  (Pawn|Input|AddControllerYawInput AxisValue))

(event Input|AxisEvents|InputAxisLookUp
  (params (AxisValue :type Float%20%28single-precision%29))
  ;[1 1 1] Camera
  (Pawn|Input|AddControllerPitchInput AxisValue))

(event Input|KeyboardEvents|O
  (params (Key :type Key%20Structure :default "None"))
  (:Pressed
    (bind _returnvalue (UserInterface|CreateWidget "/Game/Blueprints/WBP_Flash.WBP_Flash_C"))
    (UserInterface|Viewport|AddtoViewport _returnvalue 0)))

(event Input|KeyboardEvents|P
  (params (Key :type Key%20Structure :default "None"))
  (:Pressed
    (Game|SpawnActorfromClass "/Game/Blueprints/BP_Projectile.BP_Projectile_C" (Transformation|GetWorldTransform (Variables|Default|GetProjectileSpawner)) "Undefined" "MultiplyWithRoot" 0 0)))

(fn ConstructionScript)

(fn Zoomin
  (bind _camera (Variables|Default|GetCamera))
  (bind _fov_value (Variables|Default|GetFOV_Value))
  (bind _fieldofview (Variables|/Script/Engine.CameraComponent|GetFieldOfView _camera))
  (bind _returnvalue (- _fieldofview _fov_value))
  (if (<= _returnvalue (Variables|Default|GetFOV_MIN))
    (Utilities|Time|ClearTimerbyFunctionName 0 "ZoomIn")
    (else
      (Camera|SetFieldOfView _camera _returnvalue))))

(fn ZoomOut
  (bind _camera (Variables|Default|GetCamera))
  (bind _fov_value (Variables|Default|GetFOV_Value))
  (bind _fieldofview (Variables|/Script/Engine.CameraComponent|GetFieldOfView _camera))
  (bind _returnvalue (+ _fieldofview _fov_value))
  (if (>= _returnvalue (Variables|Default|GetFOX_Default))
    (Utilities|Time|ClearTimerbyFunctionName 0 "ZoomOut")
    (else
      (Camera|SetFieldOfView _camera _returnvalue))))